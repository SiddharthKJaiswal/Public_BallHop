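; BP_Ball_Base is a bouncing ball that awards score to the player character on hit.
; Static mesh hits re-apply an upward impulse with a sound, while player hits call the game mode's SpawnBall with this ball and a randomized XY transform.
; Construction derives the default impulse from spawn height, sets the material color and picks that transform.
; Two timed events temporarily boost impulse, or double scale and score, for five seconds.
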(event `self.Mesh.OnComponentHit`
  (params (HitComponent :type "PrimitiveComponent Object Reference") (OtherActor :type "Actor Object Reference") (OtherComp :type "PrimitiveComponent Object Reference") (NormalImpulse :type "Vector Structure") (Hit :type "HitResult Structure (by ref)"))
  (bind _returnvalue (`SceneComponent.K2_GetComponentLocation` (`self.ImpulsePoint`)))
  (cast `StaticMeshActor` OtherActor
    (:`then`
      (`PrimitiveComponent.AddImpulseAtLocation` (`self.Mesh`) (`self.ImpulseToAdd`) _returnvalue "None")
      (`GameplayStatics.PlaySoundAtLocation` "/Game/_BallHop/Sounds/SW_Bounce.SW_Bounce" _returnvalue (struct) 1.0 1.0 0.0 "/Game/_BallHop/Sounds/SA_Bounce.SA_Bounce" "/Game/_BallHop/Sounds/SC_Bounce.SC_Bounce" null null))
    (:`CastFailed`
      (bind _asbp_third_person_character (cast `/Game/_BallHop/Pawn/BP_ThirdPersonCharacter` OtherActor))
      (`/Game/_BallHop/Pawn/BP_ThirdPersonCharacter.UpdateScore` _asbp_third_person_character (`self.ScoreToAdd`))
      (bind _asbp_game_mode_ball_hop (cast `/Game/_BallHop/Core/BP_GameMode_BallHop` (`GameplayStatics.GetGameMode`)))
      (`/Game/_BallHop/Core/BP_GameMode_BallHop.SpawnBall` _asbp_game_mode_ball_hop (`self.DefaultTransform`) self))))

(event `AddVelocity`
  (set `self.ImpulseToAdd` (* (`self.DefaultImpulse`) 1.5))
  (`KismetSystemLibrary.Delay` 5.0)
  (set `self.ImpulseToAdd` (`self.DefaultImpulse`)))

(event `ChangeScale`
  (bind (_defaulttransform_location _defaulttransform_rotation _defaulttransform_scale) (`KismetMathLibrary.BreakTransform` (`self.DefaultTransform`)))
  (bind (_defaulttransform_location_2 _defaulttransform_rotation_2 _defaulttransform_scale_2) (`KismetMathLibrary.BreakTransform` (`self.DefaultTransform`)))
  (`self.SetActorScale3D` (* _defaulttransform_scale_2 2.0))
  (set `self.ScoreToAdd` (* (`self.ScoreToAdd`) 2))
  (`KismetSystemLibrary.Delay` 5.0)
  (`self.SetActorScale3D` _defaulttransform_scale)
  (set `self.ScoreToAdd` (/ (`self.ScoreToAdd`) 2)))

(fn `UserConstructionScript`
  (bind (_returnvalue_x _returnvalue_y _returnvalue_z) (`KismetMathLibrary.BreakVector` (`self.K2_GetActorLocation`)))
  (bind _returnvalue (`KismetMathLibrary.RandomFloatInRange` -4000.0 4000.0))
  (set `self.DefaultImpulse` (`KismetMathLibrary.MakeVector` 0.0 0.0 (* _returnvalue_z 100.0)))
  (`MeshComponent.SetVectorParameterValueOnMaterials` (`self.Mesh`) "BallColor" (`self.MaterialColor`))
  (set `self.DefaultTransform` (`KismetMathLibrary.MakeTransform` (`KismetMathLibrary.MakeVector` _returnvalue _returnvalue (.z (.location (`self.GetTransform`)))) (.rotation (`self.GetTransform`)) (.scale (`self.GetTransform`)))))