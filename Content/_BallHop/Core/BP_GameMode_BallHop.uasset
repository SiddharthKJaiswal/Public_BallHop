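; BallHop game mode that tracks the black, green and red balls and handles their respawning.
; BeginPlay caches the black ball and the green and red ball arrays.
; SpawnBall destroys a ball, then after a one-second delay spawns its class at the given transform and stores it, without removing old array entries.
; A parallel Sequence branch calls ChangeScale on every green ball when the destroyed ball is black, without waiting for the delay.
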(event `self.ReceiveBeginPlay`
  (bind _returnvalue (`GameplayStatics.GetActorOfClass` "/Game/_BallHop/Items/BP_Ball_Black.BP_Ball_Black_C"))
  (set `self.BlackBall` _returnvalue)
  (bind _outactors (`GameplayStatics.GetAllActorsOfClass` "/Game/_BallHop/Items/BP_Ball_Green.BP_Ball_Green_C"))
  (set `self.GreenBalls` _outactors)
  (bind _outactors_2 (`GameplayStatics.GetAllActorsOfClass` "/Game/_BallHop/Items/BP_Ball_Red.BP_Ball_Red_C"))
  (set `self.RedBalls` _outactors_2))

(event `SpawnBall`
  (params (SpawnTransform :type "Transform Structure") (DestroyedBallActor :type "/Game/_BallHop/Items/BP_Ball_Base Object Reference"))
  (`|ExecutionSequence`
    (:`then_0`
      (set `self.Class` (`GameplayStatics.GetObjectClass` DestroyedBallActor))
      (set `self.Transform` SpawnTransform)
      (`self.K2_DestroyActor` DestroyedBallActor)
      (`KismetSystemLibrary.Delay` 1.0)
      (`|ExecutionSequence`
        (:`then_0`
          (bind _asbp_ball_black (castclass `/Game/_BallHop/Items/BP_Ball_Black` (`self.Class`)))
          (bind _returnvalue (`|SpawnActorFromClass` _asbp_ball_black (`self.Transform`) "Undefined" "MultiplyWithRoot" null null))
          (set `self.BlackBall` _returnvalue))
        (:`then_1`
          (bind _asbp_ball_green (castclass `/Game/_BallHop/Items/BP_Ball_Green` (`self.Class`)))
          (bind _returnvalue_2 (`|SpawnActorFromClass` _asbp_ball_green (`self.Transform`) "Undefined" "MultiplyWithRoot" null null))
          (`KismetArrayLibrary.Array_Add` (`self.GreenBalls`) _returnvalue_2))
        (:`then_2`
          (bind _asbp_ball_red (castclass `/Game/_BallHop/Items/BP_Ball_Red` (`self.Class`)))
          (bind _returnvalue_3 (`|SpawnActorFromClass` _asbp_ball_red (`self.Transform`) "Undefined" "MultiplyWithRoot" null null))
          (`KismetArrayLibrary.Array_Add` (`self.RedBalls`) _returnvalue_3))))
    (:`then_1`
      (cast `/Game/_BallHop/Items/BP_Ball_Black` DestroyedBallActor)
      (for _array_element (`self.GreenBalls`)
        (`/Game/_BallHop/Items/BP_Ball_Base.ChangeScale` _array_element)))))

(fn `UserConstructionScript`)